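; BP_Romero_BT1 is a Level 2 enemy, apparently for a behavior tree version of Romero, with melee attack and death drop events.
; Attack starts a zombie punch montage, then line traces forward with persistent debug drawing and directly reduces BP_Player2_GUN's Health on a hit.
; DeathPickUp passes a DoOnce, then spawns ammo at the mesh's PickUps socket if Health is depleted.
; Neither event is called within this graph.
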(event `DeathPickUp`
  (`/Engine/EditorBlueprintResources/StandardMacros.DoOnce` false
    (:`Completed`
      (if (<= (`self.Health`) 0.0)
        (`|SpawnActorFromClass` "/Game/Assets/Ammo/Ammo_Pickups.Ammo_Pickups_C" (`KismetMathLibrary.MakeTransform` (.location (`SceneComponent.GetSocketTransform` (`self.Mesh`) "PickUps" "RTS_World")) (.rotation (`SceneComponent.GetSocketTransform` (`self.Mesh`) "PickUps" "RTS_World"))) "Undefined" "OverrideRootScale" null null)))))

(event `Attack`
  (bind _returnvalue (`self.K2_GetActorLocation`))
  (`|PlayMontage` (`self.Mesh`) "/Game/AI/Enemy/Level2/Romero_BT_Version/Animations/Zombie_Punch_Montage.Zombie_Punch_Montage"
    (:`then`
      (bind _outhit (`KismetSystemLibrary.LineTraceSingle` :`Start` _returnvalue :`End` (+ _returnvalue (* (`self.GetActorForwardVector`) 250.0)) :`TraceChannel` "TraceTypeQuery1" :`DrawDebugType` "Persistent"))
      (bind _asbp_player_2_gun (cast `/Game/ThirdPersonBP/Player/Player/BP_Player2_Gun/BP_Player2_GUN` (`.HitActor` (`GameplayStatics.BreakHitResult` _outhit))))
      (set `/Game/ThirdPersonBP/Player/Player/BP_Player2_Gun/BP_Player2_GUN.Health` (- (`/Game/ThirdPersonBP/Player/Player/BP_Player2_Gun/BP_Player2_GUN.Health` _asbp_player_2_gun) 0.5) _asbp_player_2_gun))))

(fn `UserConstructionScript`)